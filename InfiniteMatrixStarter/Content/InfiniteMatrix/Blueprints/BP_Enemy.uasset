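; BP_Enemy is an enemy actor that damages the player on contact and awards score when shot.
; All logic runs from the EnemyMesh begin-overlap event, which casts the other actor to player and projectile in sequence.
; A player hit reduces health, destroys the enemy and triggers death and restart display when health runs out.
; A projectile hit adds score through the projectile's player reference, then destroys both actors.
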(event `self.EnemyMesh.OnComponentBeginOverlap`
  (params (OverlappedComponent :type "PrimitiveComponent Object Reference") (OtherActor :type "Actor Object Reference") (OtherComp :type "PrimitiveComponent Object Reference") (OtherBodyIndex :type Integer) (bFromSweep :type Boolean) (SweepResult :type "HitResult Structure (by ref)"))
  (`|ExecutionSequence`
    (:`then_0`
      ;[1 1 1] Enemy overlap player
      (bind _asbp_player (cast `/Game/InfiniteMatrix/Blueprints/BP_Player` OtherActor))
      (`/Game/InfiniteMatrix/Blueprints/BP_Player.UpdateHealth` _asbp_player -25.0)
      (`self.K2_DestroyActor`)
      (if (<= (`/Game/InfiniteMatrix/Blueprints/BP_Player.Health` _asbp_player) 0.0)
        (set `/Game/InfiniteMatrix/Blueprints/BP_Player.IsDead ` true _asbp_player)
        (`/Game/InfiniteMatrix/Blueprints/BP_Player.DisplayRestart` _asbp_player)))
    (:`then_1`
      ;[1 1 1] Enemy overlap projectile
      (bind _asbp_projectile (cast `/Game/InfiniteMatrix/Blueprints/BP_Projectile` OtherActor))
      (`/Game/InfiniteMatrix/Blueprints/BP_Player.UpdateScore` (`/Game/InfiniteMatrix/Blueprints/BP_Projectile.BP_Player` _asbp_projectile) 15)
      (`self.K2_DestroyActor` _asbp_projectile)
      (`self.K2_DestroyActor`))))

(fn `UserConstructionScript`)